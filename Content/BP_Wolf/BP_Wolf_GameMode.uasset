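; Game mode for the Wolf egg-collecting game that holds score, health, egg count and game-over state.
; BeginPlay calls StartGame, which resets score, health and the game-over flag but leaves the egg count untouched.
; EggCollected increments both score and egg count; an unconnected check for every twentieth egg has no effect.
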(event EventBeginPlay
  (Utilities|StartGame))

(fn ConstructionScript)

(fn EggCollected
  (Variables|Default|SetScore (+ (Variables|Default|GetScore) 1))
  (Variables|Default|SetEggCount (+ (Variables|Default|GetEggCount) 1)))